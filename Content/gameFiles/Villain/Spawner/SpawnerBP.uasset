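; SpawnerBP is a placeable spawner that repeatedly spawns batches of a configurable villain class at its own transform.
; BeginPlay fires the first batch immediately and caches the third-person game mode.
; After each batch, a delayed self-calling event loop spawns again while the game mode's villain count is below its maximum, otherwise polling through ShouldSpawn.
; The cap is checked only between batches, and the spawner never updates the count itself.
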(event `self.ReceiveBeginPlay`
  (`|ExecutionSequence`
    (:`then_0`
      (`self.SpawnVillain` (`self.Villain`) (`self.GetTransform`) (`self.Number Villains`)))
    (:`then_1`
      (bind _asbp_third_person_game_mode (cast `/Game/ThirdPerson/Blueprints/BP_ThirdPersonGameMode` (`GameplayStatics.GetGameMode`)))
      (set `self.gamemodeRef` _asbp_third_person_game_mode))))

(event `SpawnVillain`
  (params (Villain :type "Actor Class Reference") (SpawnTransform :type "Transform Structure") (numberVillains :type Integer))
  (bind _gamemoderef (`self.gamemodeRef`))
  (for _ (range numberVillains)
    (`|SpawnActorFromClass` Villain SpawnTransform "Undefined" "OverrideRootScale" null null))
  (`KismetSystemLibrary.Delay` (`self.spawnDelay`))
  (if (< (`/Game/ThirdPerson/Blueprints/BP_ThirdPersonGameMode.villainSpawned` _gamemoderef) (`/Game/ThirdPerson/Blueprints/BP_ThirdPersonGameMode.maxVillain` _gamemoderef))
    (`self.SpawnVillain` (`self.Villain`) (`self.GetTransform`) (`self.Number Villains`))
    (else
      (`self.shouldSpawn`))))

(event `shouldSpawn`
  (bind _gamemoderef (`self.gamemodeRef`))
  (`KismetSystemLibrary.Delay` (`self.spawnDelay`))
  (if (< (`/Game/ThirdPerson/Blueprints/BP_ThirdPersonGameMode.villainSpawned` _gamemoderef) (`/Game/ThirdPerson/Blueprints/BP_ThirdPersonGameMode.maxVillain` _gamemoderef))
    (`self.SpawnVillain` (`self.Villain`) (`self.GetTransform`) (`self.Number Villains`))
    (else
      (`self.shouldSpawn`))))

(fn `UserConstructionScript`)