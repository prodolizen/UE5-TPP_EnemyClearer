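; VillainBP is an enemy that endlessly chases the player via a self-restarting AI MoveTo, at a walk speed randomized on spawn.
; Hitting the player applies damage, gated by a DoOnce with a delayed reset and skipped once the game is over.
; Damage lowers its clamped health with hit or death sounds; death increments the player's kill count and destroys it.
; It reports its spawn and death to the game mode through SpawnVillain and DecreaseVillain.
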(event `self.ReceiveBeginPlay`
  (bind _asue_4asp_character (cast `/Game/gameFiles/Chars/Ue4ASP_Character` (`GameplayStatics.GetPlayerCharacter` 0)))
  (bind _output_get (set `self.CharacterRef` _asue_4asp_character))
  (`self.Chase Player` _output_get)
  (set `CharacterMovementComponent.MaxWalkSpeed` (select `int` (`KismetMathLibrary.RandomInteger` 3) :`0` 100.0 :`1` 200.0 :`2` 300.0 :`3` 400.0 :!type "Float (single-precision)") (`self.CharacterMovement`))
  (bind _asbp_third_person_game_mode (cast `/Game/ThirdPerson/Blueprints/BP_ThirdPersonGameMode` (`GameplayStatics.GetGameMode`)))
  (`/Game/ThirdPerson/Blueprints/BP_ThirdPersonGameMode.spawnVillain` _asbp_third_person_game_mode))

(event `Chase Player`
  (params (Player :type "/Game/gameFiles/Chars/Ue4ASP_Character Object Reference"))
  (`|AIMoveTo` self (0.0 0.0 0.0) Player
    (:`OnSuccess`
      _)
    (:`OnFail`
      _))
  (`self.Chase Player` (`self.CharacterRef`)))

(event `self.ReceiveAnyDamage`
  (params (Damage :type "Float (single-precision)") (DamageType :type "DamageType Object Reference") (InstigatedBy :type "Controller Object Reference") (DamageCauser :type "Actor Object Reference"))
  (bind _returnvalue (`self.K2_GetActorLocation`))
  (bind _output_get (set `self.Health` (`KismetMathLibrary.FClamp` (- (`self.Health`) Damage) 0.0 100.0)))
  (if (== _output_get 0.0)
    (`GameplayStatics.PlaySoundAtLocation` "/Game/gameFiles/SFX/DeathSound.DeathSound" _returnvalue (struct) 1.0 1.0 0.0 null null null null)
    (`|ExecutionSequence`
      (:`then_0`
        (bind _asue_4asp_character (cast `/Game/gameFiles/Chars/Ue4ASP_Character` (`GameplayStatics.GetPlayerCharacter` 0)))
        (`/Engine/EditorBlueprintResources/StandardMacros.IncrementInt` (`/Game/gameFiles/Chars/Ue4ASP_Character.killCount` _asue_4asp_character)
          (:`  `
            (bind _asbp_third_person_game_mode (cast `/Game/ThirdPerson/Blueprints/BP_ThirdPersonGameMode` (`GameplayStatics.GetGameMode`)))
            (`/Game/ThirdPerson/Blueprints/BP_ThirdPersonGameMode.decreaseVillain` _asbp_third_person_game_mode))))
      (:`then_1`
        (`self.K2_DestroyActor`)))
    (else
      (`GameplayStatics.PlaySoundAtLocation` "/Game/gameFiles/SFX/HitSound.HitSound" _returnvalue (struct) 1.0 1.0 0.0 null null null null))))

(event `self.ReceiveHit`
  (params (MyComp :type "PrimitiveComponent Object Reference") (Other :type "Actor Object Reference") (OtherComp :type "PrimitiveComponent Object Reference") (bSelfMoved :type Boolean) (HitLocation :type "Vector Structure") (HitNormal :type "Vector Structure") (NormalImpulse :type "Vector Structure") (Hit :type "HitResult Structure (by ref)"))
  ;[1 1 1] Player Damage
  (bind _asue_4asp_character (cast `/Game/gameFiles/Chars/Ue4ASP_Character` (`GameplayStatics.GetPlayerCharacter` 0)))
  (if (`/Game/gameFiles/Chars/Ue4ASP_Character.gameOver` _asue_4asp_character)
    _
    (elif (`self.ActorHasTag` Other "Ue4ASP_Character")
      (`/Engine/EditorBlueprintResources/StandardMacros.DoOnce` false :!label _label
        (:`Completed`
          (`GameplayStatics.ApplyDamage` _asue_4asp_character 20.0)
          (`KismetSystemLibrary.Delay` 2.0)
          (goto _label :!via `Reset`))))))

(fn `UserConstructionScript`)