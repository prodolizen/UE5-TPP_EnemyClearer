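; Ammo crate pickup that gives the player 30 ammo when they press Interact while standing near it.
; Box overlap with Ue4ASP_Character enables input and opens a gate, and leaving disables input and closes it.
; Interact passes through the gate to add to the character's Ammo, destroy the crate and play the pickup sound at the world origin.
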(event `InputAction|Interact`
  (params (Key :type "Key Structure"))
  (:`Pressed`
    (`/Engine/EditorBlueprintResources/StandardMacros.Gate` true :!label _label
      (:`Exit`
        (bind _asue_4asp_character (cast `/Game/gameFiles/Chars/Ue4ASP_Character` (`GameplayStatics.GetPlayerCharacter` 0)))
        (set `/Game/gameFiles/Chars/Ue4ASP_Character.Ammo` (+ (`/Game/gameFiles/Chars/Ue4ASP_Character.Ammo` _asue_4asp_character) 30) _asue_4asp_character)
        (`self.K2_DestroyActor`)
        (`GameplayStatics.PlaySoundAtLocation` "/Game/gameFiles/SFX/PickUpSound.PickUpSound" (0.0 0.0 0.0) (struct) 1.0 1.0 0.0 null null null null)))))

(event `self.Box.OnComponentBeginOverlap`
  (params (OverlappedComponent :type "PrimitiveComponent Object Reference") (OtherActor :type "Actor Object Reference") (OtherComp :type "PrimitiveComponent Object Reference") (OtherBodyIndex :type Integer) (bFromSweep :type Boolean) (SweepResult :type "HitResult Structure (by ref)"))
  (cast `/Game/gameFiles/Chars/Ue4ASP_Character` OtherActor)
  (`self.EnableInput` (`GameplayStatics.GetPlayerController` 0))
  (goto _label :!via `Open`))

(event `self.Box.OnComponentEndOverlap`
  (params (OverlappedComponent :type "PrimitiveComponent Object Reference") (OtherActor :type "Actor Object Reference") (OtherComp :type "PrimitiveComponent Object Reference") (OtherBodyIndex :type Integer))
  (cast `/Game/gameFiles/Chars/Ue4ASP_Character` OtherActor)
  (`self.DisableInput` (`GameplayStatics.GetPlayerController` 0))
  (goto _label :!via `Close`))

(fn `UserConstructionScript`)